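; BP_Enemy is an enemy that makes melee attacks on the player and destroys itself when its Health component reports death.
; AttackMelee waits briefly, then checks that the player's distance is at least DistanceToAttack, as the comparison is written.
; When that passes, it damages the player's tagged HealthComponent, waits again and signals attack end.
; A failed check never signals attack end.
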(event `AttackMelee`
  (bind _returnvalue (`GameplayStatics.GetPlayerCharacter` 0))
  (`KismetSystemLibrary.Delay` 0.5)
  (if (<= (`self.DistanceToAttack`) (`self.GetDistanceTo` self _returnvalue))
    (`HealthComponent.Damage` (`self.FindComponentByTag` _returnvalue "/Script/Projekt_Jez.HealthComponent" "HealthPlayer") (`self.Damage`))
    (`KismetSystemLibrary.Delay` 0.5)
    (`self.OnAttackEnd`)))

(event `self.Health.OnDead`
  (`self.K2_DestroyActor`))

(fn `UserConstructionScript`)